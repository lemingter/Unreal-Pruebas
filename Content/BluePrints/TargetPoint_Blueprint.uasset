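; TargetPoint Blueprint actor that moves back and forth continuously between two fixed limits on the world Y axis.
; Each Tick, the Direction flag selects the Izquierda (left) or Derecha (right) vector, scales it by Speed and delta time, and applies a swept move.
; Crossing either hardcoded Y bound flips the flag.
; The transform is built from location alone, so rotation and scale are not carried over.
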(event EventBeginPlay)

(event Collision|EventActorBeginOverlap
  (params (OtherActor :type Actor%20Object%20Reference)))

(event EventTick
  (params (DeltaSeconds :type Float%20%28single-precision%29))
  (if (Variables|Default|GetDirection)
    (Transformation|SetActorTransform (Math|Conversions|ToTransform(Vector) (+ (Transformation|GetActorLocation) (* (Variables|Default|GetIzquierda) (Variables|Default|GetSpeed) (Utilities|Time|GetWorldDeltaSeconds)))) true)
    (Math|Float|CompareFloat (.y (Transformation|GetActorLocation)) -2e+02
      (:<
        (Variables|Default|SetDirection false)))
    (else
      (Transformation|SetActorTransform (Math|Conversions|ToTransform(Vector) (+ (Transformation|GetActorLocation) (* (Variables|Default|GetDerecha) (Variables|Default|GetSpeed) (Utilities|Time|GetWorldDeltaSeconds)))) true)
      (Math|Float|CompareFloat (.y (Transformation|GetActorLocation)) 1e+03
        (:>
          (Variables|Default|SetDirection true))))))

(fn ConstructionScript)